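; BP_Spawner2 is a spawner actor that scatters BP_Item actors in a box-shaped volume around itself when play begins.
; A loop driven by SpawnCount picks a random point within Scalemax half-extents and spawns with random roll and yaw, ignoring collisions.
; Each pass also removes NewVar0 from OutActors, though nothing here fills that array.
; The Box component's extent and Scalemin are unused.
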(event `self.ReceiveBeginPlay`
  (bind _returnvalue (`KismetMathLibrary.RandomFloatInRange` 0.0 359.0))
  (for _ (range (+ (`self.Spawn count`) 1))
    (`|SpawnActorFromClass` "/Game/Bluprints/ObjectGenerator/BP_Item.BP_Item_C" (`KismetMathLibrary.MakeTransform` (`KismetMathLibrary.RandomPointInBoundingBox` (`self.K2_GetActorLocation`) (`self.Scalemax`)) (`KismetMathLibrary.MakeRotator` _returnvalue 0.0 _returnvalue)) "AlwaysSpawn" "MultiplyWithRoot" null null)
    (`KismetArrayLibrary.Array_RemoveItem` (`self.Out Actors`) (`self.NewVar_0`))))

(fn `UserConstructionScript`)