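; BP_ScatterTool is an unfinished object scatter actor with variables for spawn area, count, seed, mesh and scale range.
; On BeginPlay it clears the ISMObjects instances and spawns one StaticMeshActor at a point built from random unit-vector components, without using SpawnArea.
; The count loop, bounds query and random-rotation spawn are disconnected, seed and scale inputs are unused, and the construction script is empty.
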(event `self.ReceiveBeginPlay`
  (bind (_returnvalue_x _returnvalue_y _returnvalue_z) (`KismetMathLibrary.BreakVector` (`KismetMathLibrary.RandomUnitVector`)))
  (`InstancedStaticMeshComponent.ClearInstances` (`self.ISM_Objects`))
  (`|SpawnActorFromClass` "/Script/Engine.StaticMeshActor" (`KismetMathLibrary.MakeTransform` (`KismetMathLibrary.RandomPointInBoundingBox` (`KismetMathLibrary.MakeVector` _returnvalue_x _returnvalue_y _returnvalue_z))) "AdjustIfPossibleButAlwaysSpawn" "MultiplyWithRoot" null null))

(fn `UserConstructionScript`)